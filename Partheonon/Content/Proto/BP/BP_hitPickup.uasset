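; Prototype pickup sphere that dissolves and destroys itself when the player character hits it.
; BeginPlay creates a dynamic dissolve material, with parameters set through DynaMatChange.
; A player hit clears IsPlayer and plays a timeline that animates the dissolve, then destroys the actor.
; Tick orbits the actor around the player using timeline sine/cosine offsets while IsPlayer is true, though nothing here sets that flag true.
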(event OnComponentHit(Sphere1)
  (params (HitComponent :type Primitive%20Component%20Object%20Reference) (OtherActor :type Actor%20Object%20Reference) (OtherComp :type Primitive%20Component%20Object%20Reference) (NormalImpulse :type Vector :default "0, 0, 0") (Hit :type Hit%20Result%20Structure%20%28by%20ref%29))
  ;[1 1 1] 히트 된 대상(other)가 플레이어라면
  (bind _asbp_third_person_character (Utilities|Casting|CastToBP_ThirdPersonCharacter (Game|GetPlayerCharacter 0)))
  (if (== OtherActor _asbp_third_person_character)
    (Variables|Default|Setis%20Player false)
    (bind _dissolve (Timeline|dyMatTimeLine Play)
      (:Update
        (Utilities|DynaMatChange _dissolve 0.1 1e+01))
      (:Finished
        (Actor|DestroyActor)))))

(event Custom|FollowUp
  ;[1 1 1] 나(픽업오브젝트, self)의 위치를 (플레이어 앞으로) 업데이트  해라!
  (Transformation|SetActorLocation (+ (Transformation|GetActorLocation (Game|GetPlayerCharacter 0)) (* (Variables|Default|GetroundVector) 1.1e+02)) true false))

(event EventBeginPlay
  ;[1 1 1] I will Change to Parameter in Material
  (bind _returnvalue (Rendering|Material|CreateDynamicMaterialInstance (Variables|Default|GetSphere) 0 "/Game/Proto/Materials/M_dissolve.M_dissolve" "None" :!class /Script/Engine.PrimitiveComponent))
  (Variables|Default|SetDissolveMat _returnvalue)
  (Utilities|DynaMatChange 1.0 0.05 1e+01))

(event Collision|EventActorBeginOverlap
  (params (OtherActor :type Actor%20Object%20Reference)))

(event EventTick
  (params (DeltaSeconds :type Float%20%28single-precision%29))
  ;[1 1 1] 플레이어의 정면 방향을 받아온다!
  (Utilities|FlowControl|Sequence
    (:then_0
      (if (Variables|Default|Getis%20Player) ; 플레이어가 픽업했을때만
        (CallFunction|FollowUp)))
    (:then_1
      ;[1 1 1] 플레이어 주변을 따라 도는 좌표
      (bind (_direction _sin _cos) (Timeline|Timeline Play)
        (:Update
          (Variables|Default|SetroundVector (Math|Vector|MakeVector _sin _cos 0.0)))))))

(fn ConstructionScript)